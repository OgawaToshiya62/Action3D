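; BP_Player is the playable character Blueprint, driven by Enhanced Input through the IM_Controls mapping context added on BeginPlay.
; Separate forward and strafe actions move it relative to control yaw, scaled by a Speed variable.
; Look input turns the controller and then clamps pitch to limit the camera.
; Jump triggers the character jump, and left click plays the Attack_MTG montage on the mesh.
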(event Input|EnhancedActionEvents|EnhancedInputActionIA_Jump
  (params (ActionValue :type Boolean) (ElapsedSeconds :type Float%20%28double-precision%29) (TriggeredSeconds :type Float%20%28double-precision%29) (InputAction :type Input%20Action%20Object%20Reference :default "/Game/Input/Action/IA_Jump.IA_Jump"))
  ;[0.15 0.15 0.15 0.5] ジャンプ
  (Character|Jump))

(event Input|EnhancedActionEvents|EnhancedInputActionIA_MouseL
  (params (ActionValue :type Boolean) (ElapsedSeconds :type Float%20%28double-precision%29) (TriggeredSeconds :type Float%20%28double-precision%29) (InputAction :type Input%20Action%20Object%20Reference :default "/Game/Input/Action/IA_MouseL.IA_MouseL"))
  ;[0.15 0.15 0.15 0.5] 左クリックでの攻撃
  (Animation|Montage|PlayMontage (Variables|Character|GetMesh) "/Game/Characters/Animations/MaenoAnim/Attack_MTG.Attack_MTG"))

(event Input|EnhancedActionEvents|EnhancedInputActionIA_MoveWS
  (params (ActionValue :type Float%20%28double-precision%29) (ElapsedSeconds :type Float%20%28double-precision%29) (TriggeredSeconds :type Float%20%28double-precision%29) (InputAction :type Input%20Action%20Object%20Reference :default "/Game/Input/Action/IA_MoveWS.IA_MoveWS"))
  ;[0.15 0.15 0.15 0.5] 移動
  (Pawn|Input|AddMovementInput (Math|Vector|GetForwardVector (Math|Rotator|MakeRotator 0.0 0.0 (.yaw (Pawn|GetControlRotation :!class /Script/Engine.Pawn)))) (* ActionValue (Variables|Default|GetSpeed)) false))

(event Input|EnhancedActionEvents|EnhancedInputActionIA_MoveAD
  (params (ActionValue :type Float%20%28double-precision%29) (ElapsedSeconds :type Float%20%28double-precision%29) (TriggeredSeconds :type Float%20%28double-precision%29) (InputAction :type Input%20Action%20Object%20Reference :default "/Game/Input/Action/IA_MoveAD.IA_MoveAD"))
  ;[0.15 0.15 0.15 0.5] 移動
  (Pawn|Input|AddMovementInput (Math|Vector|GetRightVector (Math|Rotator|MakeRotator 0.0 0.0 (.yaw (Pawn|GetControlRotation :!class /Script/Engine.Pawn)))) (* ActionValue (Variables|Default|GetSpeed)) false))

(event Input|EnhancedActionEvents|EnhancedInputActionIA_Look
  (params (ActionValue :type Vector%202D%20Structure) (ElapsedSeconds :type Float%20%28double-precision%29) (TriggeredSeconds :type Float%20%28double-precision%29) (InputAction :type Input%20Action%20Object%20Reference :default "/Game/Input/Action/IA_Look.IA_Look"))
  (bind (_x _y) (Math|Vector2D|BreakVector2D ActionValue))
  (bind _returnvalue (Pawn|GetControlRotation :!class /Script/Engine.Pawn))
  (bind (_roll _pitch _yaw) (Math|Rotator|BreakRotator _returnvalue))
  ;[0.15 0.15 0.15 0.5] 視点操作
  ;;[0.15 0.15 0.15 0.5] コントローラーの角度を変更する
  (Utilities|FlowControl|Sequence
    (:then_0
      (Pawn|Input|AddControllerYawInput _x)
      (Pawn|Input|AddControllerPitchInput _y))
    (:then_1
      ;;[0.15 0.15 0.15 0.5] カメラの操作を制限する
      (Pawn|SetControlRotation (Game|GetPlayerController 0) (Math|Rotator|MakeRotator 0.0 (Math|Float|ClampAngle _pitch -8e+01 3e+01) _yaw)))))

(event EventBeginPlay
  (bind _returnvalue (Game|GetPlayerController 0))
  (bind _returnvalue_2 (PlayerController|LocalPlayerSubsystems|GetEnhancedInputLocalPlayerSubsystem _returnvalue))
  ;[0.15 0.15 0.15 0.5] Input方法をIM_Controlに設定する
  (Utilities|IsValid _returnvalue_2
    (:Is%20Valid
      (Input|AddMappingContext _returnvalue_2 "/Game/Input/IM_Controls.IM_Controls" 0 "(bIgnoreAllPressedKeysUntilRelease=True,bForceImmediately=False,bNotifyUserSettings=False)"))))

(event Collision|EventActorBeginOverlap
  (params (OtherActor :type Actor%20Object%20Reference)))

(event EventTick
  (params (DeltaSeconds :type Float%20%28single-precision%29)))

(fn ConstructionScript)